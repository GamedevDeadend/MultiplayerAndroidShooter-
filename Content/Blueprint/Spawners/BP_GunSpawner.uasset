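; Weapon spawner actor that places a random gun at its own transform on BeginPlay.
; SpawnNewWeapon picks uniformly among six weapon Blueprints (pistol, assault rifle variants, rocket launcher, sniper rifle) and stores the result in SpawnedWeapon.
; A looping timer runs CheckForRespawn every ten seconds, spawning a replacement once that weapon has left the spawner's exact location.
; If SpawnedWeapon is no longer valid, no replacement spawns.
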(event `self.ReceiveBeginPlay`
  (`self.SpawnNewWeapon`)
  (`KismetSystemLibrary.K2_SetTimer` null "CheckForRespawn" 10.0 true))

(fn `CheckForRespawn`
  (bind _spawnedweapon (`self.SpawnedWeapon`)
    (:`then`
      (if (not (== (`self.K2_GetActorLocation` _spawnedweapon) (`self.K2_GetActorLocation`)))
        (`self.SpawnNewWeapon`)))
    (:`else`)))

(fn `SpawnNewWeapon`
  (bind _returnvalue (`self.GetTransform`))
  (switch `int` (`KismetMathLibrary.RandomInteger` 6)
    (:`0`
      (bind _returnvalue_2 (`|SpawnActorFromClass` "/Game/Blueprint/Weapons/HitScanWeapons/BP_Pistol.BP_Pistol_C" _returnvalue "Undefined" "OverrideRootScale" null null))
      (set `self.SpawnedWeapon` _returnvalue_2))
    (:`1`
      (bind _returnvalue_3 (`|SpawnActorFromClass` "/Game/Blueprint/Weapons/ProjectileWeapons/BP_AR_Auto.BP_AR_Auto_C" _returnvalue "Undefined" "OverrideRootScale" null null))
      (set `self.SpawnedWeapon` _returnvalue_3))
    (:`2`
      (bind _returnvalue_4 (`|SpawnActorFromClass` "/Game/Blueprint/Weapons/ProjectileWeapons/BP_AR_Burst.BP_AR_Burst_C" _returnvalue "Undefined" "OverrideRootScale" null null))
      (set `self.SpawnedWeapon` _returnvalue_4))
    (:`3`
      (bind _returnvalue_5 (`|SpawnActorFromClass` "/Game/Blueprint/Weapons/ProjectileWeapons/BP_AR_Single.BP_AR_Single_C" _returnvalue "Undefined" "OverrideRootScale" null null))
      (set `self.SpawnedWeapon` _returnvalue_5))
    (:`4`
      (bind _returnvalue_6 (`|SpawnActorFromClass` "/Game/Blueprint/Weapons/ProjectileWeapons/BP_RocketLauncher.BP_RocketLauncher_C" _returnvalue "Undefined" "OverrideRootScale" null null))
      (set `self.SpawnedWeapon` _returnvalue_6))
    (:`5`
      (bind _returnvalue_7 (`|SpawnActorFromClass` "/Game/Blueprint/Weapons/HitScanWeapons/BP_SniperRifle.BP_SniperRifle_C" _returnvalue "Undefined" "OverrideRootScale" null null))
      (set `self.SpawnedWeapon` _returnvalue_7))))

(fn `UserConstructionScript`)