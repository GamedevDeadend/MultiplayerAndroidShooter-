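; BP_MPPlayer is a player character Blueprint whose only active logic presents the sniper scope when OnScopingSniper fires.
; Aiming shows a lazily created, cached scope widget with a zoom-in animation and sound, and enables the level's first-found PostProcessVolume, also cached.
; Releasing aim starts the animation in reverse with a zoom-out sound, then immediately disables the volume and removes the widget, provided a volume is found.
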(event `self.ReceiveActorBeginOverlap`
  (params (OtherActor :type "Actor Object Reference")))

(event `self.OnScopingSniper`
  (params (isAiming :type Boolean))
  (bind _snipingwidget (`self.SnipingWidget`))
  (if isAiming
    (`self.SnipingWidget`
      (:`then`
        _)
      (:`else`
        (bind _returnvalue (`|CreateWidget` "/Game/Blueprint/WidgetsAndHUD/WBP_SniperScope.WBP_SniperScope_C"))
        (set `self.SnipingWidget` _returnvalue)))
    (`UserWidget.AddToViewport` (`self.SnipingWidget`) 0)
    (`UserWidget.PlayAnimation` (`self.SnipingWidget`) (`/Game/Blueprint/WidgetsAndHUD/WBP_SniperScope.ScopeZoomIn` (`self.SnipingWidget`)) 0.0 1 "Forward" 1.0 false)
    (`GameplayStatics.PlaySound2D` "/Game/Assets/MilitaryWeapSilver/Sound/SniperRifle/Cues/SniperRifle_ZoomIn_Cue.SniperRifle_ZoomIn_Cue" 1.0 1.0 0.0 null null)
    (`self.PP_Volume`
      (:`then`
        (set `PostProcessVolume.bEnabled` true (`self.PP_Volume`) :!label _label))
      (:`else`
        (bind _outactors (`GameplayStatics.GetAllActorsOfClass` "/Script/Engine.PostProcessVolume"))
        (if (not (`KismetArrayLibrary.Array_IsEmpty` _outactors))
          (set `self.PP_Volume` (`|GetArrayItem` _outactors))
          (goto _label))))
    (else
      (`self.SnipingWidget`
        (:`then`
          (`UserWidget.PlayAnimation` _snipingwidget (`/Game/Blueprint/WidgetsAndHUD/WBP_SniperScope.ScopeZoomIn` _snipingwidget) 0.0 1 "Reverse" 1.0 false)
          (`GameplayStatics.PlaySound2D` "/Game/Assets/MilitaryWeapSilver/Sound/SniperRifle/Wavs/SniperRifle_ZoomOut.SniperRifle_ZoomOut" 1.0 1.0 0.0 null null)
          (`self.PP_Volume`
            (:`then`
              (set `PostProcessVolume.bEnabled` false (`self.PP_Volume`) :!label _label_2)
              (`Widget.RemoveFromParent` (`self.SnipingWidget`)))
            (:`else`
              (bind _outactors_2 (`GameplayStatics.GetAllActorsOfClass` "/Script/Engine.PostProcessVolume"))
              (if (not (`KismetArrayLibrary.Array_IsEmpty` _outactors_2))
                (set `self.PP_Volume` (`|GetArrayItem` _outactors_2))
                (goto _label_2)))))
        (:`else`)))))

(fn `UserConstructionScript`)